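; AViSAvatar is an AViSCharacter child Blueprint for an avatar meant to show webcam face imagery on its head, and it sets VideoTexture to Face2 on BeginPlay.
; The parent's ServerSend stores the bitmap in FacePixels, then calls ServerSendFrame, which calls MulticastFrame.
; MulticastFrame only prints a debug message.
; Unconnected nodes sketch a dynamic M_WebCam material on Head fed by a texture imported from a buffer.
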(event Custom|MulticastFrame
  (Development|PrintText "You have been MULTICASTED"))

(event Custom|ServerSendFrame
  (CallFunction|MulticastFrame))

(event EventBeginPlay
  (Variables|Default|SetVideoTexture "/Game/face2.face2"))

(event EventServerSend
  (params (Bitmap :type Array%20of%20Color%20Structures))
  ;[1 1 1] Called from parent class, AViSCharacter
  (Variables|Default|SetFacePixels Bitmap)
  (CallFunction|ServerSendFrame))

(fn ConstructionScript)