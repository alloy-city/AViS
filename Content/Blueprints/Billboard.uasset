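; Billboard actor that appears meant to show a webcam video texture on its Billboard component, though that logic is currently unwired.
; Disconnected nodes would create a dynamic M_WebCam material and feed VideoTexture into its Texture parameter, alongside dedicated-server and CameraOn checks.
; BeginPlay and OnNextVideoFrame are empty, so the only live behavior is a debug print when C is pressed.
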(event EventBeginPlay)

(event Collision|EventActorBeginOverlap
  (params (OtherActor :type Actor%20Object%20Reference)))

(event EventTick
  (params (DeltaSeconds :type Float%20%28single-precision%29)))

(event EventOnNextVideoFrame)

(event Input|KeyboardEvents|C
  (params (Key :type Key%20Structure))
  (:Pressed
    (Development|PrintText "C")))

(fn ConstructionScript)